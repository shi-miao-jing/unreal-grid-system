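; BP_Character is the player character that moves a placement preview to the grid-snapped point where the camera is aimed.
; On BeginPlay it finds and caches the BP_GridSystem and BP_Preview actors in the level.
; Each Tick it line-traces forward from FollowCamera, with debug drawing on.
; On a hit, the grid system converts the location to a snapped tile position, and the preview actor moves there.
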(event EventBeginPlay
  (Utilities|FlowControl|Sequence
    (:then_0
      (bind _returnvalue (Actor|GetActorOfClass "/Game/BP_GridSystem.BP_GridSystem_C"))
      (Variables|Default|SetREF%20BP%20GridSystem _returnvalue))
    (:then_1
      (bind _returnvalue_2 (Actor|GetActorOfClass "/Game/BP_Preview.BP_Preview_C"))
      (Variables|Default|SetREF%20BP%20Preview _returnvalue_2))))

(event EventTick
  (params (DeltaSeconds :type Float%20%28single-precision%29))
  (bind _followcamera (Variables|Default|GetFollowCamera))
  (bind _returnvalue (Transformation|GetWorldLocation _followcamera))
  (bind (_outhit _returnvalue_2) (Collision|LineTraceByChannel _returnvalue (+ _returnvalue (* (Math|Vector|GetForwardVector _followcamera) (Variables|Default|GetTraceDistance))) "TraceTypeQuery1" false 0 "ForOneFrame"))
  (if _returnvalue_2
    (bind _returnvalue_3 (Class|GridSystem|GetSnapLocation :self (Variables|Default|GetREF%20BP%20GridSystem) :HitLocation (.location _outhit)))
    (Transformation|SetActorLocation (Variables|Default|GetREF%20BP%20Preview) _returnvalue_3 false false)))

(fn ConstructionScript)